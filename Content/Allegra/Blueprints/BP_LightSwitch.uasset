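; Light switch actor that toggles a linked light source's point light on the Interact input action.
; ToggleLight swaps the switch mesh material between green and red, flips SwitchOn, then sets the point light's visibility to match.
; The material is chosen before the flip, so green ends up showing with the light off and red with it on.
; The graph has no proximity or target check.
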(event Input|EnhancedActionEvents|EnhancedInputActionIA_Interact
  (params (ActionValue :type Boolean) (ElapsedSeconds :type Float%20%28double-precision%29) (TriggeredSeconds :type Float%20%28double-precision%29) (InputAction :type Input%20Action%20Object%20Reference :default "/Game/Input/Actions/IA_Interact.IA_Interact"))
  (:Triggered
    (CallFunction|ToggleLight)))

(fn ConstructionScript)

(fn ToggleLight
  (bind _lightswitchmesh (Variables|Default|GetLightswitchMesh))
  (if (Variables|Default|GetbSwitchOn)
    (Rendering|Material|SetMaterial _lightswitchmesh 0 "/Game/Allegra/Materials/M_Green.M_Green")
    (else
      (Rendering|Material|SetMaterial _lightswitchmesh 0 "/Game/Allegra/Materials/M_Red.M_Red")))
  (bind _output_get (Variables|Default|SetbSwitchOn (not (Variables|Default|GetbSwitchOn))))
  (Rendering|SetVisibility (Variables|/Game/Allegra/Blueprints/BP_LightSource.BP_LightSource_C|GetPointLight (Variables|Default|GetLightSource)) _output_get false))