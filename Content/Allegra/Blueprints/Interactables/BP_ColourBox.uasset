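; Grabbable colour puzzle box that changes and mixes colour when it overlaps BP_ColourChanger actors.
; Gameplay tags track the current colour: red, blue and yellow pairs mix into purple, green or orange, and white resets it.
; A mixed box records a MixedColours tag and ignores further colours except white.
; Colour shows through a dynamic material parameter, and interaction calls GrabRelease on the first-person character.
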(event OnComponentBeginOverlap(MoveableBoxCollision)
  (params (OverlappedComponent :type Primitive%20Component%20Object%20Reference) (OtherActor :type Actor%20Object%20Reference) (OtherComp :type Primitive%20Component%20Object%20Reference) (OtherBodyIndex :type Integer) (bFromSweep :type Boolean) (SweepResult :type Hit%20Result%20Structure%20%28by%20ref%29))
  ;[0.15 0.15 0.15 0.5] Box Colour Change On Overlap
  (bind _asbp_colour_changer (Utilities|Casting|CastToBP_ColourChanger OtherActor))
  (if (GameplayTags|MatchesTag (Variables|/Game/Allegra/Blueprints/Triggers/BP_ColourChanger.BP_ColourChanger_C|GetColourTags _asbp_colour_changer) "(TagName=\"Puzzle.Colour.White\")")
    (Variables|Default|SetCurrentColourTag "(TagName=\"Puzzle.Colour.White\")")
    (Variables|Default|SetIsMixedColour false)
    (CallFunction|ColourChanging :!label _label)
    (elif (not (Variables|Default|GetIsMixedColour))
      (|SwitchGameplayTag (Variables|/Game/Allegra/Blueprints/Triggers/BP_ColourChanger.BP_ColourChanger_C|GetColourTags _asbp_colour_changer)
        (:Puzzle.Colour.Red
          (CallFunction|RedMixOptions)
          (goto _label))
        (:Puzzle.Colour.Blue
          (CallFunction|BlueMixOptions)
          (goto _label))
        (:Puzzle.Colour.White
          (Variables|Default|SetCurrentColourTag "(TagName=\"Puzzle.Colour.White\")")
          (goto _label))
        (:Puzzle.Colour.Yellow
          (CallFunction|YellowMixOptions)
          (goto _label))))))

(event EventBeginPlay
  (bind _cubemesh (Variables|Default|GetCubeMesh))
  (bind _returnvalue (Rendering|Material|CreateDynamicMaterialInstance _cubemesh 0 (Rendering|Material|GetMaterial _cubemesh 0) "None" :!class /Script/Engine.PrimitiveComponent))
  (Variables|Default|SetCubeMaterial _returnvalue))

(event EventTriggerInteraction
  (params (Interactor :type Actor%20Object%20Reference))
  ;[0.15 0.15 0.15 0.5] Grab/Release Event
  (bind _asbp_first_person_character (Utilities|Casting|CastToBP_FirstPersonCharacter Interactor))
  (Default|GrabRelease _asbp_first_person_character))

(fn ConstructionScript)

(fn ColourChanging
  (|SwitchGameplayTag (Variables|Default|GetCurrentColourTag)
    (:Puzzle.Colour.Blue
      (Colours|ChangeBlue))
    (:Puzzle.Colour.Yellow
      (Colours|ChangeYellow))
    (:Puzzle.Colour.Red
      (Colours|ChangeRed))
    (:Puzzle.Colour.White
      (Colours|ChangeWhite))
    (:Puzzle.Colour.Purple
      (Colours|ChangePurple))
    (:Puzzle.Colour.Green
      (Colours|ChangeGreen))
    (:Puzzle.Colour.Orange
      (Colours|ChangeOrange))))

(fn ChangeBlue
  (Variables|Default|SetCubeMaterial (Variables|Default|GetCubeMaterial))
  (Rendering|Material|SetVectorParameterValue (Variables|Default|GetCubeMaterial) "BaseColour" (Variables|Colours|GetBlue) :!class /Script/Engine.MaterialInstanceDynamic))

(fn ChangeYellow
  (Variables|Default|SetCubeMaterial (Variables|Default|GetCubeMaterial))
  (Rendering|Material|SetVectorParameterValue (Variables|Default|GetCubeMaterial) "BaseColour" (Variables|Colours|GetYellow) :!class /Script/Engine.MaterialInstanceDynamic))

(fn ChangeRed
  (Variables|Default|SetCubeMaterial (Variables|Default|GetCubeMaterial))
  (Rendering|Material|SetVectorParameterValue (Variables|Default|GetCubeMaterial) "BaseColour" (Variables|Colours|GetRed) :!class /Script/Engine.MaterialInstanceDynamic))

(fn ChangePurple
  (Variables|Default|SetCubeMaterial (Variables|Default|GetCubeMaterial))
  (Rendering|Material|SetVectorParameterValue (Variables|Default|GetCubeMaterial) "BaseColour" (Variables|Colours|GetPurple) :!class /Script/Engine.MaterialInstanceDynamic)
  (Variables|Default|SetMixedColoursTag "(TagName=\"MixedColours.Box.Purple\")")
  (Variables|Default|SetIsMixedColour true))

(fn ChangeGreen
  (Variables|Default|SetCubeMaterial (Variables|Default|GetCubeMaterial))
  (Rendering|Material|SetVectorParameterValue (Variables|Default|GetCubeMaterial) "BaseColour" (Variables|Colours|GetGreen) :!class /Script/Engine.MaterialInstanceDynamic)
  (Variables|Default|SetMixedColoursTag "(TagName=\"MixedColours.Box.Green\")")
  (Variables|Default|SetIsMixedColour true))

(fn ChangeWhite
  (Variables|Default|SetCubeMaterial (Variables|Default|GetCubeMaterial))
  (Rendering|Material|SetVectorParameterValue (Variables|Default|GetCubeMaterial) "BaseColour" (Variables|Colours|GetWhite) :!class /Script/Engine.MaterialInstanceDynamic))

(fn YellowMixOptions
  (|SwitchGameplayTag (Variables|Default|GetCurrentColourTag)
    (:Default
      (Variables|Default|SetCurrentColourTag "(TagName=\"Puzzle.Colour.Yellow\")"))
    (:Puzzle.Colour.Blue
      (Variables|Default|SetCurrentColourTag "(TagName=\"Puzzle.Colour.Green\")"))
    (:Puzzle.Colour.Red
      (Variables|Default|SetCurrentColourTag "(TagName=\"Puzzle.Colour.Orange\")"))))

(fn BlueMixOptions
  (|SwitchGameplayTag (Variables|Default|GetCurrentColourTag)
    (:Default
      (Variables|Default|SetCurrentColourTag "(TagName=\"Puzzle.Colour.Blue\")"))
    (:Puzzle.Colour.Red
      (Variables|Default|SetCurrentColourTag "(TagName=\"Puzzle.Colour.Purple\")"))
    (:Puzzle.Colour.Yellow
      (Variables|Default|SetCurrentColourTag "(TagName=\"Puzzle.Colour.Green\")"))))

(fn RedMixOptions
  (|SwitchGameplayTag (Variables|Default|GetCurrentColourTag)
    (:Default
      (Variables|Default|SetCurrentColourTag "(TagName=\"Puzzle.Colour.Red\")"))
    (:Puzzle.Colour.Blue
      (Variables|Default|SetCurrentColourTag "(TagName=\"Puzzle.Colour.Purple\")"))
    (:Puzzle.Colour.Yellow
      (Variables|Default|SetCurrentColourTag "(TagName=\"Puzzle.Colour.Orange\")"))))

(fn ChangeOrange
  (Variables|Default|SetCubeMaterial (Variables|Default|GetCubeMaterial))
  (Rendering|Material|SetVectorParameterValue (Variables|Default|GetCubeMaterial) "BaseColour" (Variables|Colours|GetOrange) :!class /Script/Engine.MaterialInstanceDynamic)
  (Variables|Default|SetMixedColoursTag "(TagName=\"MixedColours.Box.Orange\")")
  (Variables|Default|SetIsMixedColour true))

(fn GetInteractionPrompt
  (return ""))