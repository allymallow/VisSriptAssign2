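; BP_HitPlate is a trigger plate that reacts when a BP_PhysicsOrb enters its Sphere collision.
; If HasDoorTrigger is set, the hit calls DoorActivated on the referenced DoorToActivate; otherwise it spawns NS_Sparks at the plate mesh's location.
; On BeginPlay it applies its Material variable to the plate mesh.
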(event OnComponentBeginOverlap(Sphere)
  (params (OverlappedComponent :type Primitive%20Component%20Object%20Reference) (OtherActor :type Actor%20Object%20Reference) (OtherComp :type Primitive%20Component%20Object%20Reference) (OtherBodyIndex :type Integer) (bFromSweep :type Boolean) (SweepResult :type Hit%20Result%20Structure%20%28by%20ref%29))
  ;[0.15 0.15 0.15 0.5] Door Open/Close
  (Utilities|Casting|CastToBP_PhysicsOrb OtherActor)
  (if (Variables|Default|GetHasDoorTrigger)
    (Default|DoorActivated (Variables|Default|GetDoorToActivate))
    (else
      (Niagara|SpawnSystematLocation "/Game/Allegra/Feedback/Visual/NS_Sparks.NS_Sparks" (Transformation|GetWorldLocation (Variables|Default|GetPlateMesh))))))

(event EventBeginPlay
  (Rendering|Material|SetMaterial (Variables|Default|GetPlateMesh) 0 (Variables|Default|GetMaterial)))

(fn ConstructionScript)