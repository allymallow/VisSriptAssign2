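; Pressure plate that activates its linked door when a BP_ColourBox with the matching colour overlaps it.
; On BeginPlay it creates a dynamic material on the plate mesh and tints it with its in-game colour.
; Overlap compares the box's mixed-colour tag to TagToOpen; no end-overlap logic exists here.
; A separate state setter, not called within this Blueprint, swaps the plate to white, red, blue or yellow materials.
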(event EventBeginPlay
  (bind _returnvalue (Rendering|Material|CreateDynamicMaterialInstance (Variables|Default|GetPlateMesh) 0 (Variables|MaterialandColour|GetSource%20Material) "None" :!class /Script/Engine.PrimitiveComponent))
  (bind _output_get (Variables|MaterialandColour|SetMaterialReference _returnvalue))
  (Rendering|Material|SetVectorParameterValue _output_get "BaseColour" (Variables|MaterialandColour|GetInGameColour) :!class /Script/Engine.MaterialInstanceDynamic))

(event Collision|EventActorBeginOverlap
  (params (OtherActor :type Actor%20Object%20Reference))
  ;[0.15 0.15 0.15 0.5] Door Open/Close
  (bind _asbp_colour_box (Utilities|Casting|CastToBP_ColourBox OtherActor))
  (if (== (Variables|/Game/Allegra/Blueprints/Interactables/BP_ColourBox.BP_ColourBox_C|GetMixedColoursTag _asbp_colour_box) (Variables|Default|GetTagToOpen))
    (Default|DoorActivated (Variables|Default|GetDoorToActivate))))

(fn ConstructionScript)

(fn SetNewState
  (params (CurrentState :type E_PressurePlateState%20Enum :default "NewEnumerator0"))
  (bind _platemesh (Variables|Default|GetPlateMesh))
  (bind _output_get (Variables|Default|SetCurrentState CurrentState))
  (switch Utilities|FlowControl|Switch|SwitchonE_PressurePlateState _output_get
    (:NewEnumerator1
      (Rendering|Material|SetMaterial (Variables|Default|GetPlateMesh) 0 "/Game/Allegra/Materials/M_White.M_White"))
    (:NewEnumerator2
      (Rendering|Material|SetMaterial _platemesh 0 "/Game/Allegra/Materials/M_Red.M_Red"))
    (:NewEnumerator3
      (Rendering|Material|SetMaterial _platemesh 0 "/Game/Allegra/Materials/M_Blue.M_Blue"))
    (:NewEnumerator4
      (Rendering|Material|SetMaterial _platemesh 0 "/Game/Allegra/Materials/M_Yellow.M_Yellow"))))

(fn GetCurrentState
  (return (Variables|Default|GetCurrentState)))