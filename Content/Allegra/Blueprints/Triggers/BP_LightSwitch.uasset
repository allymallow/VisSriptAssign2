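; BP_LightSwitch is an interactable wall switch that turns three referenced scene lights on and off.
; BeginPlay gathers the light references into an array.
; TriggerInteraction calls ToggleLight, which plays a sound at the switch mesh, flips SwitchOn and sets each light's root component visibility without propagating to children.
; An IsInteracting flag with a short delay debounces repeated presses, and the interaction prompt is empty.
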(event EventBeginPlay
  (Variables|Default|SetLightsInScene (Utilities|Array|MakeArray (Variables|Default|GetLight1) (Variables|Default|GetLight2) (Variables|Default|GetLight3))))

(event EventTriggerInteraction
  (params (Interactor :type Actor%20Object%20Reference))
  (if (not (Variables|Default|GetIsInteracting))
    (Variables|Default|SetIsInteracting true)
    (CallFunction|ToggleLight)
    (Utilities|FlowControl|Delay 0.5)
    (Variables|Default|SetIsInteracting false)))

(fn ConstructionScript)

(fn ToggleLight
  (Audio|PlaySoundatLocation (Variables|Default|GetSound) (Transformation|GetWorldLocation (Variables|Default|GetLightSwitchMesh)) "0, 0, 0" 1.0 1.0 0.0 0 0 0 0)
  (bind _output_get (Variables|Default|SetSwitchOn (not (Variables|Default|GetSwitchOn))))
  (for _array_element (Variables|Default|GetLightsInScene)
    (Rendering|SetVisibility (Variables|/Script/Engine.Actor|GetRootComponent _array_element) _output_get false)))

(fn GetInteractionPrompt
  (return ""))