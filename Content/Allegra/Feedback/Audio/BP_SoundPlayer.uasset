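; BP_SoundPlayer is a feedback actor that plays sounds for colour box matches and door movement.
; When a BP_ColourBox enters its Trigger, it compares the box's MixedColoursTag with TagToTrigger, non-exact, and plays a positive or negative sound.
; DoorOpen and DoorClose events play their own sounds.
; All sounds share one SFXPlayer component, whose sound is swapped before each play.
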(event OnComponentBeginOverlap(Trigger)
  (params (OverlappedComponent :type Primitive%20Component%20Object%20Reference) (OtherActor :type Actor%20Object%20Reference) (OtherComp :type Primitive%20Component%20Object%20Reference) (OtherBodyIndex :type Integer) (bFromSweep :type Boolean) (SweepResult :type Hit%20Result%20Structure%20%28by%20ref%29))
  (bind _sfxplayer (Variables|Default|GetSFXPlayer))
  (bind _sfxplayer_2 (Variables|Default|GetSFXPlayer))
  (bind _asbp_moveable_box (Utilities|Casting|CastToBP_ColourBox OtherActor))
  (if (GameplayTags|MatchesTag (Variables|/Game/Allegra/Blueprints/Interactables/BP_ColourBox.BP_ColourBox_C|GetMixedColoursTag _asbp_moveable_box) (Variables|Default|GetTagToTrigger))
    (Audio|Components|Audio|SetSound _sfxplayer (Variables|Default|GetPosSFXToPlay))
    (Audio|Components|Audio|Play _sfxplayer 0.0)
    (else
      (Audio|Components|Audio|SetSound _sfxplayer_2 (Variables|Default|GetNegSFXToPlay_0))
      (Audio|Components|Audio|Play _sfxplayer_2 0.0))))

(event Custom|DoorOpen
  (bind _sfxplayer (Variables|Default|GetSFXPlayer))
  (Audio|Components|Audio|SetSound _sfxplayer (Variables|Default|GetDoorOpenPlay))
  (Audio|Components|Audio|Play _sfxplayer 0.0))

(event Custom|DoorClose
  (bind _sfxplayer (Variables|Default|GetSFXPlayer))
  (Audio|Components|Audio|SetSound _sfxplayer (Variables|Default|GetDoorClosePlay))
  (Audio|Components|Audio|Play _sfxplayer 0.0))

(fn ConstructionScript)